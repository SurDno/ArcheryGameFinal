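; BP_EnemyTestAI is a simple enemy that chases the player on sight and returns to its spawn location.
; PawnSensing resets a last-seen timer, and Tick issues AI MoveTo toward the player for a few seconds before heading home.
; Hitting the player reduces their health and destroys the enemy.
; A projectile hit destroys both projectile and enemy.
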(event OnSeePawn(PawnSensing)
  (params (Pawn :type Pawn%20Object%20Reference))
  (Utilities|Casting|CastToBP_FirstPersonCharacter Pawn)
  (Variables|Default|SetiTimeSinceLastSeen 0.0))

(event EventBeginPlay
  (Variables|Default|SetHomePosition (Transformation|GetActorLocation)))

(event EventTick
  (params (DeltaSeconds :type Float%20%28single-precision%29))
  (if (< (Variables|Default|GetiTimeSinceLastSeen) 3.0)
    (Variables|Default|SetiTimeSinceLastSeen (+ DeltaSeconds (Variables|Default|GetiTimeSinceLastSeen) 0.0))
    (AI|AIMoveTo self "0, 0, 0" (Game|GetPlayerCharacter 0) 0.0 false)
    (else
      (AI|AIMoveTo self (Variables|Default|GetHomePosition) 0 5.0 false))))

(event Collision|EventHit
  (params (MyComp :type Primitive%20Component%20Object%20Reference) (Other :type Actor%20Object%20Reference) (OtherComp :type Primitive%20Component%20Object%20Reference) (bSelfMoved :type Boolean) (HitLocation :type Vector :default "0, 0, 0") (HitNormal :type Vector :default "0, 0, 0") (NormalImpulse :type Vector :default "0, 0, 0") (Hit :type Hit%20Result%20Structure%20%28by%20ref%29))
  (bind _asbp_first_person_character (Utilities|Casting|CastToBP_FirstPersonCharacter Other)
    (:then
      (Default|DecreaseHealth _asbp_first_person_character 0.35))
    (:CastFailed
      (bind _asbp_first_person_projectile (Utilities|Casting|CastToBP_FirstPersonProjectile Other))
      (Actor|DestroyActor _asbp_first_person_projectile)))
  (Actor|DestroyActor))

(fn ConstructionScript)